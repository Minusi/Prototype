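; BP_HelperGamemode is a game mode Blueprint in the RuntimeGizmo import's Maps folder, with no active logic.
; Its event graph holds only a disconnected debug snippet that deprojects the mouse position to a world direction, prints it and draws it as an arrow.
; Unused nodes for direction length, mouse delta and camera transform remain, and the construction script is empty.
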(fn ConstructionScript)