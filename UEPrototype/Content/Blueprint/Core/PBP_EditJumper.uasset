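; PBP_EditJumper is an actor that glides a given Subject actor to a spot just short of a Target actor.
; JumpToTarget disables the subject's collision and sets the endpoint at the target's bounds center, pulled back along the approach direction by scaled extent length.
; Tick blends start to end through the SpeedGraph curve over RunningTime, then restores collision and releases the subject.
; Invalid subjects or targets only print a screen message.
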(event Custom|JumpToTarget
  (params (Subject :type Actor%20Object%20Reference) (Target :type Actor%20Object%20Reference))
  (bind (_origin _boxextent) (Collision|GetActorBounds Target false))
  ;[1 1 1] 점프 대상 지정 후 초기화
  (Utilities|IsValid Subject
    (:Is%20Valid
      (bind _output_get (Variables|대상(custom)|SetNowMovingActor Subject)) ; 움직이는 대상 설정
      (Utilities|IsValid Target
        (:Is%20Valid
          (Collision|SetActorEnableCollision _output_get false) ; 충돌 끄기
          (Variables|위치(custom)|SetStartPoint (Transformation|GetActorLocation _output_get)) ; 시작점
          (Variables|위치(custom)|SetEndPoint (- _origin (* (Math|Vector|Normalize (- _origin (Transformation|GetActorLocation _output_get))) (* (Math|Float|Absolute(Float) (Math|Vector|VectorLength _boxextent)) (Variables|위치(custom)|GetConstant))))) ; 종료지점
          (Variables|시간(custom)|SetTimeFactor 0.0) ; 시간 초기화
        )
        (:Is%20Not%20Valid
          (Class|MinusiFrameworkLibrary|ScreenLog "Invalid Target(s)" "(R=243,G=156,B=18,A=255)" :!label _label) ; 예외처리
        )))
    (:Is%20Not%20Valid
      (goto _label))))

(event EventBeginPlay)

(event Collision|EventActorBeginOverlap
  (params (OtherActor :type Actor%20Object%20Reference)))

(event EventTick
  (params (DeltaSeconds :type Float%20%28single-precision%29))
  ;[1 1 1] 틱 당 현재 이동 액터 이동
  (if (> 1.0 (Variables|시간(custom)|GetTimeFactor)) ; 돌아가는지 확인
    (Utilities|IsValid (Variables|대상(custom)|GetNowMovingActor)
      (:Is%20Valid
        (Transformation|SetActorLocation (Variables|대상(custom)|GetNowMovingActor) (+ (* (Variables|위치(custom)|GetStartPoint) (- 1.0 (Math|Curves|GetFloatValue (Variables|대상(custom)|GetSpeedGraph) (stale _output_get)))) (* (Variables|위치(custom)|GetEndPoint) (Math|Curves|GetFloatValue (Variables|대상(custom)|GetSpeedGraph) (stale _output_get)))) false false) ; 진행도에 따라 이동
      )
      (:Is%20Not%20Valid
        _))
    (bind _output_get (Variables|시간(custom)|SetTimeFactor (+ (stale _output_get) (/ DeltaSeconds (Variables|시간(custom)|GetRunningTime))))) ; 진행도 진행
    (else
      (Utilities|IsValid (Variables|대상(custom)|GetNowMovingActor) ; 작업중이던 친구 있는지
        (:Is%20Valid
          (Collision|SetActorEnableCollision (Variables|대상(custom)|GetNowMovingActor) true) ; 다시 충돌 켜주기
          (Variables|대상(custom)|SetNowMovingActor 0) ; 오브젝트 클리어
        )))))

(fn ConstructionScript)