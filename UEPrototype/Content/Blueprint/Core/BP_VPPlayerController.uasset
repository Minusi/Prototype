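; Player controller that passes movement, look and focus input to the VP director pawn.
; On BeginPlay it casts and caches the controlled director pawn, printing a message if the cast fails.
; The three move axes share one local-axis MoveAround call, noted as XY in VR and XYZ on desktop, while desktop look axes rotate the pawn.
; A per-tick focus event forwards its target to the editor focus interpreter when valid.
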(event EventBeginPlay
  ;[1 1 1] 블루프린트 변수 초기화
  (bind _asvpdirector_pawn (Utilities|Casting|CastToVPDirectorPawn (Pawn|GetControlledPawn))
    (:then
      (Variables|Core|Player|SetVPDirectorPawn _asvpdirector_pawn))
    (:CastFailed
      (Development|PrintString "DirectorPawn이 유효하지 않습니다"))))

(event EventFocusEvent
  (params (Target :type Actor%20Object%20Reference) (DeltaTime :type Float%20%28single-precision%29))
  (bind _editorfocusmetainputinterpreter (Variables|Default|GetEditorFocusMetaInputInterpreter))
  ;[1 1 1] Focus 이벤트(매 Tick마다 호출)
  (Utilities|IsValid _editorfocusmetainputinterpreter
    (:Is%20Valid
      (Class|EditorFocusMetaInputInterpreter|InterpreteFocus _editorfocusmetainputinterpreter Target DeltaTime))))

(event Input|ActionEvents|InputActionMainFunction
  (params (Key :type Key%20Structure)))

(event Input|AxisEvents|InputAxisMoveRight
  (params (AxisValue :type Float%20%28single-precision%29))
  ;[1 1 1] 이동(VR : XY 지원, 데스크탑 : XYZ 지원)
  (Class|VPDirectorPawn|MoveAround (Variables|Core|Player|GetVPDirectorPawn) "MT_LOCALAXIS" (stale Input|AxisEvents|InputAxisMoveForward AxisValue) AxisValue (stale Input|AxisEvents|InputAxisMoveUp AxisValue) 0))

(event Input|AxisEvents|InputAxisMoveForward
  (params (AxisValue :type Float%20%28single-precision%29))
  ;[1 1 1] 이동(VR : XY 지원, 데스크탑 : XYZ 지원)
  (Class|VPDirectorPawn|MoveAround (Variables|Core|Player|GetVPDirectorPawn) "MT_LOCALAXIS" AxisValue (stale Input|AxisEvents|InputAxisMoveRight AxisValue) (stale Input|AxisEvents|InputAxisMoveUp AxisValue) 0))

(event Input|AxisEvents|InputAxisLookUp
  (params (AxisValue :type Float%20%28single-precision%29))
  ;[1 1 1] 회전 (데스크탑 전용)
  (Class|VPDirectorPawn|LookUpSide (Variables|Core|Player|GetVPDirectorPawn) AxisValue))

(event Input|AxisEvents|InputAxisLookSide
  (params (AxisValue :type Float%20%28single-precision%29))
  ;[1 1 1] 회전 (데스크탑 전용)
  (Class|VPDirectorPawn|LookSide (Variables|Core|Player|GetVPDirectorPawn) AxisValue))

(event Input|AxisEvents|InputAxisMoveUp
  (params (AxisValue :type Float%20%28single-precision%29))
  ;[1 1 1] 이동(VR : XY 지원, 데스크탑 : XYZ 지원)
  (Class|VPDirectorPawn|MoveAround (Variables|Core|Player|GetVPDirectorPawn) "MT_LOCALAXIS" (stale Input|AxisEvents|InputAxisMoveForward AxisValue) (stale Input|AxisEvents|InputAxisMoveRight AxisValue) AxisValue 0))

(fn ConstructionScript)