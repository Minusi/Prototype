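; Transform gizmo axes actor that tracks the currently selected actor while the gizmo is activated.
; Each tick it teleports to the selected actor's location, without sweeping.
; It also scales uniformly with the distance between that actor and the player pawn, within a clamped range, to offset perspective shrinking.
; The scale is only rewritten when it differs from the current one beyond a small tolerance.
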(event EventBeginPlay)

(event Collision|EventActorBeginOverlap
  (params (OtherActor :type Actor%20Object%20Reference)))

(event EventTick
  (params (DeltaSeconds :type Float%20%28single-precision%29))
  (bind _returnvalue (Game|Player|GetPlayerPawn 0))
  (bind _selectedactor (Variables|Default|GetSelectedActor))
  (bind _returnvalue_2 (Transformation|GetDistanceTo _selectedactor _returnvalue))
  (bind _returnvalue_3 (* _returnvalue_2 0.0005))
  (bind _returnvalue_4 (+ _returnvalue_3 0.9))
  (bind _returnvalue_5 (Math|Float|Clamp(Float) _returnvalue_4 1.0 4.0))
  (if (and (Variables|Default|GetbIsGizmoActivated) (Utilities|IsValid _selectedactor))
    (Transformation|SetActorLocation (Transformation|GetActorLocation _selectedactor) false true)
    (if (not (Math|Float|NearlyEqual(Float) _returnvalue_5 (.x (Transformation|GetActorScale3D)) 0.001))
      (Transformation|SetActorScale3D (* "1.000000,1.000000,1.000000" _returnvalue_5)))))

(fn ConstructionScript)